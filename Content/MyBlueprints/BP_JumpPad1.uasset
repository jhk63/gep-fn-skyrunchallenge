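; BP_JumpPad1 is a jump pad that launches the third-person character when it enters the pad's box trigger.
; On overlap it adds an impulse along the Arrow component's forward vector, scaled by JumpForce, as a velocity change that ignores mass.
; Two MoveComponentTo nodes that would lower and raise the blue spring platform are left unconnected, so they never run.
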(event OnComponentBeginOverlap(Box)
  (params (OverlappedComponent :type Primitive%20Component%20Object%20Reference) (OtherActor :type Actor%20Object%20Reference) (OtherComp :type Primitive%20Component%20Object%20Reference) (OtherBodyIndex :type Integer) (bFromSweep :type Boolean) (SweepResult :type Hit%20Result%20Structure%20%28by%20ref%29))
  (bind _asbp_third_person_character (Utilities|Casting|CastToBP_ThirdPersonCharacter OtherActor))
  (Physics|AddImpulse (Variables|/Script/Engine.Character|GetCharacterMovement _asbp_third_person_character) (* (Math|Vector|GetForwardVector (Variables|Default|GetArrow)) (Variables|Default|GetJumpForce)) true))

(event OnComponentEndOverlap(Box)
  (params (OverlappedComponent :type Primitive%20Component%20Object%20Reference) (OtherActor :type Actor%20Object%20Reference) (OtherComp :type Primitive%20Component%20Object%20Reference) (OtherBodyIndex :type Integer)))

(fn ConstructionScript)