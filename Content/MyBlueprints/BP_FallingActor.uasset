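; BP_FallingActor is a platform that falls after the player character steps into its trigger box, then resets itself.
; On overlap with BP_ThirdPersonCharacter, it waits a configurable Duration, then enables physics simulation on the Platfrombigred component so it drops.
; Three seconds later it disables physics and teleports the platform back to the location and rotation of the Respawn component.
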(event OnComponentBeginOverlap(Box)
  (params (OverlappedComponent :type Primitive%20Component%20Object%20Reference) (OtherActor :type Actor%20Object%20Reference) (OtherComp :type Primitive%20Component%20Object%20Reference) (OtherBodyIndex :type Integer) (bFromSweep :type Boolean) (SweepResult :type Hit%20Result%20Structure%20%28by%20ref%29))
  (bind _platfrombigred (Variables|Default|Getplatfrombigred))
  (bind _respawn (Variables|Default|GetRespawn))
  (Utilities|Casting|CastToBP_ThirdPersonCharacter OtherActor)
  (Utilities|FlowControl|Delay (Variables|Default|GetDuration))
  (Physics|SetSimulatePhysics _platfrombigred true)
  (Utilities|FlowControl|Delay 3.0)
  (Physics|SetSimulatePhysics _platfrombigred false)
  (Transformation|SetWorldLocationAndRotation _platfrombigred (Transformation|GetWorldLocation _respawn) (Transformation|GetWorldRotation _respawn) false true))

(fn ConstructionScript)