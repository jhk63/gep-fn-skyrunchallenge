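; BP_SuperJump is a spring platform that gives the third-person character a much higher jump while standing on it.
; Box overlap begin and end events tween the spring mesh between a lowered and a raised relative position with MoveComponentTo.
; After casting to BP_ThirdPersonCharacter, they boost the character's JumpZVelocity on entry and set it back to a hardcoded lower value on exit.
; The mesh moves for any overlapping actor, since the cast follows the move.
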(event OnComponentBeginOverlap(Box)
  (params (OverlappedComponent :type Primitive%20Component%20Object%20Reference) (OtherActor :type Actor%20Object%20Reference) (OtherComp :type Primitive%20Component%20Object%20Reference) (OtherBodyIndex :type Integer) (bFromSweep :type Boolean) (SweepResult :type Hit%20Result%20Structure%20%28by%20ref%29))
  (Components|MoveComponentTo (Variables|Default|Getplatformspringblue) "0.000000,0.000000,-30.000000" "0, 0, 0" true false 0.1 false)
  (bind _asbp_third_person_character (Utilities|Casting|CastToBP_ThirdPersonCharacter OtherActor))
  (Variables|/Script/Engine.CharacterMovementComponent|SetJumpZVelocity (Variables|/Script/Engine.Character|GetCharacterMovement _asbp_third_person_character) 2e+03))

(event OnComponentEndOverlap(Box)
  (params (OverlappedComponent :type Primitive%20Component%20Object%20Reference) (OtherActor :type Actor%20Object%20Reference) (OtherComp :type Primitive%20Component%20Object%20Reference) (OtherBodyIndex :type Integer))
  (Components|MoveComponentTo (Variables|Default|Getplatformspringblue) "0.000000,0.000000,30.000000" "0, 0, 0" true false 0.1 false)
  (bind _asbp_third_person_character (Utilities|Casting|CastToBP_ThirdPersonCharacter OtherActor))
  (Variables|/Script/Engine.CharacterMovementComponent|SetJumpZVelocity (Variables|/Script/Engine.Character|GetCharacterMovement _asbp_third_person_character) 7e+02))

(fn ConstructionScript)