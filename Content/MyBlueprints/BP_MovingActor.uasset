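; BP_MovingActor is an actor whose Platformred component eases back and forth between two points, PosA and PosB.
; On BeginPlay it snaps Platformred to PosA's world location and starts an endless loop.
; A FlipFlop alternates MoveComponentTo calls toward each point's relative location over MovingTime, with a one-second Delay before looping back.
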(event EventBeginPlay
  (Transformation|SetWorldLocation (Variables|Default|Getplatformred) (Transformation|GetWorldLocation (Variables|Default|GetposA)) false false)
  (Utilities|FlowControl|FlipFlop :!label _label
    (:A
      (Components|MoveComponentTo (Variables|Default|Getplatformred) (Variables|/Script/Engine.SceneComponent|GetRelativeLocation (Variables|Default|GetPosB)) "0, 0, 0" true true (Variables|Default|GetMovingTime) false))
    (:B
      (Components|MoveComponentTo (Variables|Default|Getplatformred) (Variables|/Script/Engine.SceneComponent|GetRelativeLocation (Variables|Default|GetPosA)) "0, 0, 0" true true (Variables|Default|GetMovingTime) false)))
  (Utilities|FlowControl|Delay 1.0)
  (goto _label))

(fn ConstructionScript)